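; Game state Blueprint for Rhythm of the Demon that switches UI screens and input mode as the game changes state.
; BeginPlay creates one MainWidget, and events display its menu, game, pause, win and lose widgets, with end animatics replacing win at level index 3.
; DisplayGameUI feeds player, enemy, rhythm and scoring references into the game widget.
; Pause and resume blend cameras; resume runs a countdown before restarting music unless the tutorial freezes time.
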(event `self.Win_Event`
  (bind _mainwidget (`self.MainWidget`))
  (bind _mainwidget_2 (`self.MainWidget`))
  (`|ExecutionSequence`
    (:`then_0`
      (`WidgetBlueprintLibrary.SetInputMode_UIOnlyEx` (`GameplayStatics.GetPlayerController` 0) null))
    (:`then_1`
      (`WidgetBlueprintLibrary.SetInputMode_UIOnlyEx` (`GameplayStatics.GetPlayerController` 1) null))
    (:`then_2`
      (if (== (`self.GetCurrentLevelIndex`) 3)
        (`/Game/Blueprints/UI/ReworkUI/MainWidget.DisplayWidget` _mainwidget_2 (`/Game/Blueprints/UI/ReworkUI/MainWidget.EndAnimaticsWidget` _mainwidget_2) false)
        (else
          (`/Game/Blueprints/UI/ReworkUI/MainWidget.DisplayWidget` _mainwidget (`/Game/Blueprints/UI/ReworkUI/MainWidget.WinWidget` _mainwidget) false))))))

(event `self.ReceiveBeginPlay`
  (cast `RhythmOfTheDemonGameModeBase` (`GameplayStatics.GetGameMode`))
  (bind _returnvalue (`|CreateWidget` "/Game/Blueprints/UI/ReworkUI/MainWidget.MainWidget_C"))
  (set `self.MainWidget` _returnvalue))

(event `self.InitGame_Event`
  (`UserWidget.AddToViewport` (`self.MainWidget`) 0)
  (set `LevelStreaming.bShouldBeVisible` true (`GameplayStatics.GetStreamingLevel` "Level_01_GFX")))

(event `self.Lose_Event`
  (bind _mainwidget (`self.MainWidget`))
  (`|ExecutionSequence`
    (:`then_0`
      (`WidgetBlueprintLibrary.SetInputMode_UIOnlyEx` null null))
    (:`then_1`
      (`WidgetBlueprintLibrary.SetInputMode_UIOnlyEx` null null))
    (:`then_2`
      (`/Game/Blueprints/UI/ReworkUI/MainWidget.DisplayWidget` _mainwidget (`/Game/Blueprints/UI/ReworkUI/MainWidget.LoseWidget` _mainwidget) false))))

(event `self.Pause_Event`
  (bind _mainwidget (`self.MainWidget`))
  (`|ExecutionSequence`
    (:`then_0`
      (`WidgetBlueprintLibrary.SetInputMode_UIOnlyEx` (`GameplayStatics.GetPlayerController` 0) null))
    (:`then_1`
      (`WidgetBlueprintLibrary.SetInputMode_UIOnlyEx` (`GameplayStatics.GetPlayerController` 1) null))
    (:`then_2`
      (`CameraHandler.BlendTo` (`self.m_cameraHandler`) "PAUSE" false)
      (`KismetSystemLibrary.Delay` 1.0)
      (`/Game/Blueprints/UI/ReworkUI/MainWidget.DisplayWidget` _mainwidget (`/Game/Blueprints/UI/ReworkUI/MainWidget.PauseWidget` _mainwidget) false))))

(event `self.OnLoadLevel_Event`
  (`|ExecutionSequence`
    (:`then_2`
      (`WidgetBlueprintLibrary.SetInputMode_GameOnly` (`GameplayStatics.GetPlayerController` 0)))
    (:`then_3`
      (`WidgetBlueprintLibrary.SetInputMode_GameOnly` (`GameplayStatics.GetPlayerController` 1)))
    (:`then_4`
      (`self.DisplayGameUI`))))

(event `self.DisplayMenuUI_Event`
  (bind _mainwidget (`self.MainWidget`))
  (`|ExecutionSequence`
    (:`then_0`
      (`WidgetBlueprintLibrary.SetInputMode_UIOnlyEx` (`GameplayStatics.GetPlayerController` 0) null))
    (:`then_1`
      (`WidgetBlueprintLibrary.SetInputMode_UIOnlyEx` (`GameplayStatics.GetPlayerController` 1) null))
    (:`then_2`
      (`/Game/Blueprints/UI/ReworkUI/MainWidget.DisplayWidget` _mainwidget (`/Game/Blueprints/UI/ReworkUI/MainWidget.MenuWidget` _mainwidget) false))))

(event `self.GoToMenu_Event`
  (`|ExecutionSequence`
    (:`then_0`
      (`WidgetBlueprintLibrary.SetInputMode_UIOnlyEx` (`GameplayStatics.GetPlayerController` 0) null))
    (:`then_1`
      (`WidgetBlueprintLibrary.SetInputMode_UIOnlyEx` (`GameplayStatics.GetPlayerController` 1) null))))

(event `self.Resume_Event`
  (bind _m_camerahandler (`self.m_cameraHandler`))
  (`CameraHandler.BlendTo` _m_camerahandler (`CameraHandler.GetLastCameraKey` _m_camerahandler) false)
  (`|ExecutionSequence`
    (:`then_0`
      (`WidgetBlueprintLibrary.SetInputMode_GameOnly` (`GameplayStatics.GetPlayerController` 0)))
    (:`then_1`
      (`WidgetBlueprintLibrary.SetInputMode_GameOnly` (`GameplayStatics.GetPlayerController` 1)))
    (:`then_2`
      (`KismetSystemLibrary.Delay` 1.0)
      (`self.DisplayUnpauseTimer` 3.5))
    (:`then_3`
      (`KismetSystemLibrary.Delay` 4.0)
      (bind _returnvalue (`TutorialHandler.IsTutorialFreezingTime` (`self.m_tutoHandler`)))
      (if (not _returnvalue)
        (`self.ResumeMusic`))
      (set `self.m_isPause` false)
      (`self.DisplayGameUI`))))

(fn `CreateAllWidget`)

(fn `DisplayGameUI`
  (locals (Player :type "PlayerEntity Object Reference") (Enemy :type "MiniBossPawn Object Reference") (GameWidget :type "/Game/Blueprints/UI/ReworkUI/GameWidget Object Reference"))
  (bind _mainwidget (`self.MainWidget`))
  (bind _output_get (set `local.GameWidget` (`/Game/Blueprints/UI/ReworkUI/MainWidget.GameWidget` _mainwidget)))
  (`/Game/Blueprints/UI/ReworkUI/MainWidget.DisplayWidget` _mainwidget _output_get false)
  (bind _asro_dgame_mode (cast `/Game/Blueprints/RoDGameMode` (`GameplayStatics.GetGameMode`)))
  (`|ExecutionSequence`
    (:`then_0`
      (bind _returnvalue (`RhythmOfTheDemonGameModeBase.GetPlayer` _asro_dgame_mode))
      (set `local.Player` _returnvalue))
    (:`then_1`
      (bind _returnvalue_2 (`RhythmOfTheDemonGameModeBase.GetEnemy` _asro_dgame_mode))
      (set `local.Enemy` _returnvalue_2))
    (:`then_2`
      (`/Game/Blueprints/UI/ReworkUI/GameWidget.InitSubWidget` (`local.GameWidget`) (`local.Player`) (`local.Enemy`) (`self.m_rhythmHandler`) (`self.m_scoringHandler`)))))

(fn `DisplayUnpauseTimer`
  (params (Time :type "Float (double-precision)"))
  (bind _mainwidget (`self.MainWidget`))
  (bind _timerwidget (`/Game/Blueprints/UI/ReworkUI/MainWidget.TimerWidget` _mainwidget))
  (`/Game/Blueprints/UI/ReworkUI/MainWidget.DisplayWidget` _mainwidget _timerwidget false)
  (`/Game/Blueprints/UI/ReworkUI/TimerWidget.StartTimer` _timerwidget Time))

(fn `GetLightLevelName`
  (returns (LightLevelToLoad :type Name))
  (return (`KismetStringLibrary.Conv_StringToName` (`KismetStringLibrary.Concat_StrStr` "LightLevel_lvl" (`KismetStringLibrary.Conv_IntToString` (`self.GetCurrentLevelIndex`))))))

(fn `UserConstructionScript`)