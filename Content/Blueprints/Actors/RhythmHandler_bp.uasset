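; RhythmHandler_bp is an actor Blueprint that starts and stops the ambient music.
; MusicStartEvent plays the SOUND_AMBIENCE event in 2D and stores the returned instance in AmbiantMusic, which MusicStopEvent later stops.
; A MusicPlaying flag guards both events against repeated starts or stops.
; Despite the name, it holds no rhythm or timing logic, and BeginPlay, overlap and Tick are unused.
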(event `self.MusicStartEvent`
  (if (not (`self.musicPlaying`))
    (bind _returnvalue (`FMODBlueprintStatics.PlayEvent2D` "/Game/FMOD/Events/Amb/SOUND_AMBIENCE.SOUND_AMBIENCE"))
    (set `self.AmbiantMusic` _returnvalue)
    (set `self.musicPlaying` true)))

(event `self.MusicStopEvent`
  (if (`self.musicPlaying`)
    (`FMODBlueprintStatics.EventInstanceStop` (`self.AmbiantMusic`))
    (set `self.musicPlaying` false)))

(fn `UserConstructionScript`)