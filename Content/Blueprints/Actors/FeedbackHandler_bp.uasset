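; FeedbackHandler is an actor that delivers player feedback for a two-player game with Arm and Leg roles.
; On BeginPlay it creates a FeedbackUI widget and adds it to the viewport, then forwards success or failure text events to it for the targeted player type.
; Controller shake events play a given force feedback effect on player controller 0 for Arm, 1 for Leg, or both.
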(event `self.ReceiveBeginPlay`
  (bind _returnvalue (`|CreateWidget` "/Game/Blueprints/UI/FeedbackUI/FeedbackUI.FeedbackUI_C"))
  (bind _output_get (set `self.FeedbackUI` _returnvalue))
  (`UserWidget.AddToViewport` _output_get 0))

(event `self.ShowTextFeedback`
  (params (success :type "ESUCCESS_TYPE Enum" :default "Perfect") (target :type "EPLAYER_TYPE Enum" :default "Arm"))
  (`/Game/Blueprints/UI/FeedbackUI/FeedbackUI.ShowFeedback` (`self.FeedbackUI`) target success))

(event `self.ShakeController`
  (params (target :type "EPLAYER_TYPE Enum" :default "Arm") (shakeEffect :type "ForceFeedbackEffect Object Reference"))
  (bind _returnvalue (`GameplayStatics.GetPlayerController` 0))
  (bind _returnvalue_2 (`GameplayStatics.GetPlayerController` 1))
  (switch `EPLAYER_TYPE` target
    (:`Arm`
      (`PlayerController.ClientPlayForceFeedback` _returnvalue shakeEffect false false "None"))
    (:`Leg`
      (`PlayerController.ClientPlayForceFeedback` _returnvalue_2 shakeEffect false false "None"))
    (:`Both`
      (`PlayerController.ClientPlayForceFeedback` _returnvalue shakeEffect false false "None")
      (`PlayerController.ClientPlayForceFeedback` _returnvalue_2 shakeEffect false false "None"))))

(fn `UserConstructionScript`)