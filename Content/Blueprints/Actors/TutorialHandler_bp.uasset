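; TutorialHandler_bp is an actor that drives tutorial presentation: input prompts, step feedback text and per-actor slow motion.
; On BeginPlay it creates a TutorialUI widget, adds it to the viewport with input prompts hidden, then forwards show, hide and step-text events to it.
; A single timeline, its play rate scaled by the requested duration, eases an actor's time dilation, playing forward to slow and reversing to restore.
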(event `self.ReceiveBeginPlay`
  (bind _returnvalue (`|CreateWidget` "/Game/Blueprints/UI/TutorialUI.TutorialUI_C"))
  (bind _output_get (set `self.TutoUI` _returnvalue))
  (`UserWidget.AddToViewport` _output_get 0)
  (`/Game/Blueprints/UI/TutorialUI.HideInputUI` (`self.TutoUI`)))

(event `self.ShowInputUI`
  (params (action :type "EACTION_MAPPING Enum" :default "DashVertical"))
  (`/Game/Blueprints/UI/TutorialUI.ShowInputUI` (`self.TutoUI`) action))

(event `self.HideInputUI`
  (`/Game/Blueprints/UI/TutorialUI.HideInputUI` (`self.TutoUI`)))

(event `self.SlowActorTime`
  (params (actor :type "Actor Object Reference") (duration :type "Float (single-precision)"))
  (`TimelineComponent.SetPlayRate` (`self.SlowTimeline`) (/ 1.0 duration))
  (bind (_direction _timeevolution) (`Timeline|SlowTimeline` :!label _label)
    (:`Update`
      (switch `ETimelineDirection` _direction
        (:`Forward`
          (`self.ChangeActorTimeDilatationTo` actor _timeevolution))
        (:`Backward`
          (`self.ChangeActorTimeDilatationTo` (stale `self.UnSlowActorTime` actor) _timeevolution))))))

(event `self.UnSlowActorTime`
  (params (actor :type "Actor Object Reference") (duration :type "Float (single-precision)"))
  (`TimelineComponent.SetPlayRate` (`self.SlowTimeline`) (/ 1.0 duration))
  (goto _label :!via `Reverse`))

(event `self.ShowTutoStepFeedback`
  (params (stepIdx :type Integer) (duration :type "Float (single-precision)"))
  (`/Game/Blueprints/UI/TutorialUI.ShowTutoStepText` (`self.TutoUI`) stepIdx duration))

(fn `UserConstructionScript`)