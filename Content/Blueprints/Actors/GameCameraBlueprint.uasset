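; Game camera actor with logic to keep the player framed and widen field of view with speed, though Tick is empty and that logic is unwired.
; UpdateCameraOffset nudges a target offset when the player's projected screen position leaves a central band, and MoveCamera lerps toward it.
; ComputeFOV derives a clamped FOV from speed above a reference.
; ComputeFOVLatence applies rises instantly and eases drops toward medium or minimum FOV.
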(event `self.ReceiveBeginPlay`
  (bind _asro_dgame_mode (cast `/Game/Blueprints/RoDGameMode` (`GameplayStatics.GetGameMode`)))
  (set `self.CameraHandler` (`RhythmOfTheDemonGameModeBase.m_cameraHandler` _asro_dgame_mode)))

(event `self.ReceiveTick`
  (params (DeltaSeconds :type "Float (single-precision)")))

(fn `ComputeCameraMovement`
  (if (> (`PlayerEntity.m_speed` (`self.player`)) 60.0)
    (`self.UpdateCameraOffset`)
    (`self.MoveCamera` 0.0)))

(fn `ComputeFOV`
  (locals (ReferenceSpeed :type "Float (double-precision)" :default 190.0) (DiffSpeed :type "Float (double-precision)" :default 0.0))
  (bind _player (`self.player`))
  (bind _minfov (`self.MinFOV`))
  (`/Engine/EditorBlueprintResources/StandardMacros.IsValid` _player
    (:`Is Valid`
      (bind _output_get (set `local.DiffSpeed` (- (`PlayerEntity.m_speed` _player) (`local.ReferenceSpeed`))))
      (if (> _output_get 0.0)
        (set `self.LastFOV` (`self.NewFOV`))
        (set `self.NewFOV` (`KismetMathLibrary.FClamp` (+ (* (/ (`local.DiffSpeed`) (`self.MaxFOV`)) _minfov) _minfov) (`self.MinFOV`) (`self.MaxFOV`)))))))

(fn `ComputeFOVLatence`
  (bind _returnvalue (`GameplayStatics.GetWorldDeltaSeconds`))
  (bind _newfov (`self.NewFOV`))
  (bind _cameracomponent (`self.CameraComponent`))
  (bind _fieldofview (`CameraComponent.FieldOfView` (`self.CameraComponent`)))
  (`/Engine/EditorBlueprintResources/StandardMacros.IsValid` (`self.player`)
    (:`Is Valid`
      (if (> (`self.LastFOV`) _newfov)
        (if (< (`self.NewFOV`) (`self.MedFOV`))
          (`CameraComponent.SetFieldOfView` _cameracomponent (`KismetMathLibrary.Lerp` _fieldofview (`self.MinFOV`) _returnvalue))
          (else
            (`CameraComponent.SetFieldOfView` _cameracomponent (`KismetMathLibrary.Lerp` _fieldofview (`self.MedFOV`) _returnvalue))))
        (else
          (`CameraComponent.SetFieldOfView` _cameracomponent _newfov))))))

(fn `MoveCamera`
  (params (DeltaTime :type "Float (double-precision)"))
  (bind _cameracomponent (`self.CameraComponent`))
  (`SceneComponent.K2_SetRelativeLocation` _cameracomponent (`KismetMathLibrary.VLerp` (`SceneComponent.RelativeLocation` _cameracomponent) (`self.CameraPosTarget`) (* DeltaTime (`self.CameraLerpSpeed`))) false false))

(fn `Reset`
  (`SceneComponent.K2_SetRelativeLocation` (`self.CameraComponent`) (0.0 0.0 0.0) false false)
  (set `self.CameraPosTarget` (0.0 0.0 0.0)))

(fn `SetCameraPlayerData`
  (params (Player :type "PlayerEntity Object Reference"))
  (set `self.player` Player))

(fn `UpdateCameraOffset`
  (locals (Direction :type "Vector2D Structure"))
  (bind (_returnvalue_x _returnvalue_y) (`KismetMathLibrary.BreakVector2D` (`WidgetLayoutLibrary.GetViewportSize`)))
  (bind _screenposition (`GameplayStatics.ProjectWorldToScreen` (`GameplayStatics.GetPlayerController` 0) (`SceneComponent.K2_GetComponentLocation` (`AbstractEntityActor.m_skeletalMeshComponent` (`self.player`)))))
  (bind _returnvalue (/ (`KismetMathLibrary.BreakVector2D` _screenposition) _returnvalue_x))
  (bind _returnvalue_2 (/ (`.Y` (`KismetMathLibrary.BreakVector2D` _screenposition)) _returnvalue_y))
  (`|ExecutionSequence`
    (:`then_0`
      (if (> _returnvalue 0.65)
        (set `self.CameraPosTarget` (+ (`self.CameraPosTarget`) (0.0 10.0 0.0)))))
    (:`then_1`
      (if (< _returnvalue 0.35)
        (set `self.CameraPosTarget` (+ (`self.CameraPosTarget`) (0.0 -10.0 0.0)))))
    (:`then_2`
      (if (> _returnvalue_2 0.72)
        (set `self.CameraPosTarget` (+ (`self.CameraPosTarget`) (0.0 0.0 -10.0)))))
    (:`then_3`
      (if (< _returnvalue_2 0.45)
        (set `self.CameraPosTarget` (+ (`self.CameraPosTarget`) (0.0 0.0 10.0)))))))

(fn `UserConstructionScript`)