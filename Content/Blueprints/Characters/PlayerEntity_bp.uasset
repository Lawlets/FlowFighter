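; Player entity Blueprint that drives the player's animation and cameras in the RoD game mode.
; It forwards revert, damage and dash events to PlayerAnimationBlueprint as four arm counters, hit reactions and four-way dodges chosen by dominant axis.
; Child GameCameraBlueprint actors provide quarter-right, quarter-left and front views, initialized with the player and reset between levels.
; C toggles a prototype live editor, but its setup and SwitchCameraView are disconnected stubs.
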(event `self.ReceiveBeginPlay`
  (`self.InitAnimInstance`)
  (`self.EnableInput` (`GameplayStatics.GetPlayerController` 0))
  (`self.SetupProtoLiveEditor`)
  (bind _asro_dgame_mode (cast `/Game/Blueprints/RoDGameMode` (`GameplayStatics.GetGameMode`)))
  (set `self.RotD_GameMode` _asro_dgame_mode)
  (`|ExecutionSequence`
    (:`then_0`
      (`self.SetCameraActor`))
    (:`then_1`
      (`/Game/Blueprints/Actors/GameCameraBlueprint.SetCameraPlayerData` (`self.QuarterRightCameraActor`) self))
    (:`then_2`
      (`/Game/Blueprints/Actors/GameCameraBlueprint.SetCameraPlayerData` (`self.QuarterLeftCameraActor`) self))
    (:`then_3`
      (`/Game/Blueprints/Actors/GameCameraBlueprint.SetCameraPlayerData` (`self.FrontCameraActor`) self))))

(event `Key|C`
  (params (Key :type "Key Structure"))
  (bind _protoliveeditor (`self.ProtoLiveEditor`))
  (:`Pressed`
    (if (`Widget.IsVisible` _protoliveeditor)
      (`/Game/Blueprints/UI/ProtoLiveEditor.Hide` _protoliveeditor)
      (else
        (`/Game/Blueprints/UI/ProtoLiveEditor.Show` _protoliveeditor)))))

(event `self.RevertA_Event`
  (bind _animationblueprint (`self.AnimationBlueprint`))
  (`/Engine/EditorBlueprintResources/StandardMacros.IsValid` _animationblueprint
    (:`Is Valid`
      (`/Game/Blueprints/Animation/Player/PlayerAnimationBlueprint.TopLeftArmCounter` _animationblueprint))))

(event `self.RevertB_Event`
  (bind _animationblueprint (`self.AnimationBlueprint`))
  (`/Engine/EditorBlueprintResources/StandardMacros.IsValid` _animationblueprint
    (:`Is Valid`
      (`/Game/Blueprints/Animation/Player/PlayerAnimationBlueprint.TopRightArmCounter` _animationblueprint))))

(event `self.RevertX_Event`
  (bind _animationblueprint (`self.AnimationBlueprint`))
  (`/Engine/EditorBlueprintResources/StandardMacros.IsValid` _animationblueprint
    (:`Is Valid`
      (`/Game/Blueprints/Animation/Player/PlayerAnimationBlueprint.BotLeftArmCounter` _animationblueprint))))

(event `self.RevertY_Event`
  (bind _animationblueprint (`self.AnimationBlueprint`))
  (`/Engine/EditorBlueprintResources/StandardMacros.IsValid` _animationblueprint
    (:`Is Valid`
      (`/Game/Blueprints/Animation/Player/PlayerAnimationBlueprint.BotRightArmCounter` _animationblueprint))))

(event `self.Dash_Event`
  (params (direction :type "Vector Structure"))
  (bind _animationblueprint (`self.AnimationBlueprint`))
  (if (>= (`KismetMathLibrary.Abs` direction_Y) (`KismetMathLibrary.Abs` direction_Z))
    (if (== (`KismetMathLibrary.SignOfFloat` direction_Y) 1.0)
      (`/Game/Blueprints/Animation/Player/PlayerAnimationBlueprint.DodgeRight` _animationblueprint)
      (else
        (`/Game/Blueprints/Animation/Player/PlayerAnimationBlueprint.DodgeLeft` _animationblueprint)))
    (elif (== (`KismetMathLibrary.SignOfFloat` direction_Z) 1.0)
      (`/Game/Blueprints/Animation/Player/PlayerAnimationBlueprint.DodgeTop` _animationblueprint)
      (else
        (`/Game/Blueprints/Animation/Player/PlayerAnimationBlueprint.DodgeBot` _animationblueprint)))))

(event `self.OnTakeDamage_Event`
  (`/Game/Blueprints/Animation/Player/PlayerAnimationBlueprint.TakeDamage` (`self.AnimationBlueprint`)))

(fn `CameraLookAtEnemy`
  (bind _quarterrightcameraactor (`self.QuarterRightCameraActor`))
  (bind _returnvalue (`RhythmOfTheDemonGameModeBase.GetEnemy` (`self.RotD_GameMode`)))
  (`/Engine/EditorBlueprintResources/StandardMacros.IsValid` _returnvalue
    (:`Is Valid`
      (`SceneComponent.K2_SetWorldRotation` (`Actor.RootComponent` _quarterrightcameraactor) (`KismetMathLibrary.FindLookAtRotation` (`self.K2_GetActorLocation` _quarterrightcameraactor) (`self.K2_GetActorLocation` _returnvalue)) false false))))

(fn `InitAnimInstance`
  (bind _asplayer_animation_blueprint (cast `/Game/Blueprints/Animation/Player/PlayerAnimationBlueprint` (`SkeletalMeshComponent.GetAnimInstance` (`self.m_skeletalMeshComponent`)))
    (:`then`
      (bind _output_get (set `self.AnimationBlueprint` _asplayer_animation_blueprint))
      (set `/Game/Blueprints/Animation/Player/PlayerAnimationBlueprint.PlayerEntity` self _output_get)
      (set `/Game/Blueprints/Animation/Player/PlayerAnimationBlueprint.DashSpeed` (`self.m_dashSpeed`) _asplayer_animation_blueprint))
    (:`CastFailed`
      (`KismetSystemLibrary.PrintString` "Cannot cast anim instant to PlayerAnimationBlueprint"))))

(fn `ResetBeforeNewLevel`
  (`/Game/Blueprints/Actors/GameCameraBlueprint.Reset` (`self.QuarterRightCameraActor`))
  (`/Game/Blueprints/Actors/GameCameraBlueprint.Reset` (`self.QuarterLeftCameraActor`))
  (`/Game/Blueprints/Actors/GameCameraBlueprint.Reset` (`self.FrontCameraActor`)))

(fn `SetCameraActor`
  (bind _asgame_camera_blueprint (cast `/Game/Blueprints/Actors/GameCameraBlueprint` (`self.GetQuarterRightCameraChildActor`)))
  (set `self.QuarterRightCameraActor` _asgame_camera_blueprint)
  (bind _asgame_camera_blueprint_2 (cast `/Game/Blueprints/Actors/GameCameraBlueprint` (`self.GetQuarterLeftCameraChildActor`)))
  (set `self.QuarterLeftCameraActor` _asgame_camera_blueprint_2)
  (bind _asgame_camera_blueprint_3 (cast `/Game/Blueprints/Actors/GameCameraBlueprint` (`self.GetMenuCameraChildActor`)))
  (set `self.FrontCameraActor` _asgame_camera_blueprint_3))

(fn `SetupProtoLiveEditor`)

(fn `SwichToQuarterCamera`
  (`PlayerController.SetViewTargetWithBlend` (`GameplayStatics.GetPlayerController` 0) (`ChildActorComponent.ChildActor` (`self.m_pauseCameraActorComponent`)) 1.0 "VTBlend_Linear" 0.0 false))

(fn `SwitchCameraView`
  (params (camera_type :type Byte)))

(fn `UserConstructionScript`)