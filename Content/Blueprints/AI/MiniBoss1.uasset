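; MiniBoss1 is a mini-boss Blueprint that forwards combat events to its apostle animation Blueprint and dynamic tattoo material.
; Cast bricks select left or right projectile and obstacle animations by class.
; Damage updates the Mantra child actor's life display and flashes the tattoo red before restoring cached values.
; Overkill and death timelines drive glow parameters, with montages for death and revive.
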(event `self.ReceiveBeginPlay`
  (bind _asanimation_blueprint_apostle_lvl_1 (cast `/Game/Blueprints/Animation/AI/Apostle_lvl1/AnimationBlueprint_apostle_lvl1` (`SkeletalMeshComponent.GetAnimInstance` (`self.m_skeletalMeshComponent`))))
  (bind _output_get (set `self.AnimationBlueprint` _asanimation_blueprint_apostle_lvl_1))
  (set `/Game/Blueprints/Animation/AI/Apostle_lvl1/AnimationBlueprint_apostle_lvl1.ApostleEntity` self _output_get))

(event `self.OnMatInstanciated`
  (bind _returnvalue (`MaterialInstanceDynamic.K2_GetVectorParameterValue` (`self.m_dynamicMaterial`) "Tattoo color"))
  (set `self.TattooEmissiveColor` _returnvalue)
  (bind _returnvalue_2 (`MaterialInstanceDynamic.K2_GetScalarParameterValue` (`self.m_dynamicMaterial`) "Tattoo Power"))
  (set `self.TattooPower` _returnvalue_2))

(event `self.ReceiveTick`
  (params (DeltaSeconds :type "Float (single-precision)")))

(event `self.OnTakeDamage_Event`
  (bind _asmantra_blueprint (cast `/Game/ART/Characters/MantraBlueprint` (`ChildActorComponent.ChildActor` (`self.mantra`))))
  (`/Game/ART/Characters/MantraBlueprint.UpdateBossMantra` _asmantra_blueprint (`self.m_life`) (`self.m_lifeMax`) (`self.m_maxOverkillValue`))
  (`/Game/Blueprints/Animation/AI/Apostle_lvl1/AnimationBlueprint_apostle_lvl1.TakeDamage` (`self.AnimationBlueprint`))
  (`self.DamageFeedback`))

(event `self.CastProjEvent`
  (params (brick :type "AbstractBrick Object Reference"))
  (`self.PlayAnimationFromBrickType` brick))

(event `DamageFeedback`
  (bind _m_dynamicmaterial (`self.m_dynamicMaterial`))
  (`MaterialInstanceDynamic.SetVectorParameterValue` _m_dynamicmaterial "Tattoo color" (struct :`R` 1.0 :`B` 0.01271 :`A` 1.0))
  (`MaterialInstanceDynamic.SetScalarParameterValue` _m_dynamicmaterial "Tattoo Power" 300.0)
  (`KismetSystemLibrary.Delay` 1.0)
  (`MaterialInstanceDynamic.SetVectorParameterValue` _m_dynamicmaterial "Tattoo color" (`self.TattooEmissiveColor`))
  (`MaterialInstanceDynamic.SetScalarParameterValue` _m_dynamicmaterial "Tattoo Power" (`self.TattooPower`)))

(event `self.OnOverkill`
  (bind _m_dynamicmaterial (`self.m_dynamicMaterial`))
  (`ActorComponent.Activate` (`self.OverkillFX`) true)
  (bind (_direction _overkillprogress) (`Timeline|OverkillTimeline`)
    (:`Update`
      (`MaterialInstanceDynamic.SetScalarParameterValue` _m_dynamicmaterial "Overkill" _overkillprogress))
    (:`Finished`
      (bind _returnvalue (`MaterialInstanceDynamic.K2_GetScalarParameterValue` _m_dynamicmaterial "Tattoo Power"))
      (set `self.TattooPower` _returnvalue)
      (`MaterialInstanceDynamic.K2_GetVectorParameterValue` _m_dynamicmaterial "Tattoo color"))))

(event `OnDearth`
  (bind _m_dynamicmaterial (`self.m_dynamicMaterial`))
  (if (<= (`self.m_life`) 0.0)
    (`|PlayMontage` (`self.m_skeletalMeshComponent`) "/Game/Blueprints/Animation/AI/Apostle_lvl1/Montages/Death_Montage.Death_Montage"
      (:`then`
        (bind _returnvalue (`MaterialInstanceDynamic.K2_GetScalarParameterValue` _m_dynamicmaterial "Fresnel Power Overkill"))
        (set `self.OnDeathFresnelPower` _returnvalue)
        (bind _returnvalue_2 (`MaterialInstanceDynamic.K2_GetScalarParameterValue` _m_dynamicmaterial "Tattoo Power Overkill"))
        (bind _output_get (set `self.OnDeathTattooPower` _returnvalue_2))
        (`KismetSystemLibrary.PrintString` (`KismetStringLibrary.Conv_DoubleToString` _output_get))
        (bind (_direction _progress) (`Timeline|DeathTimeline` :!via `PlayFromStart`)
          (:`Update`
            (`MaterialInstanceDynamic.SetScalarParameterValue` _m_dynamicmaterial "Fresnel Power Overkill" (`KismetMathLibrary.Lerp` (`self.OnDeathFresnelPower`) 0.0 _progress))
            (`MaterialInstanceDynamic.SetScalarParameterValue` _m_dynamicmaterial "Tattoo Power Overkill" (`KismetMathLibrary.Lerp` (`self.OnDeathTattooPower`) 0.0 _progress))))))))

(event `OnRevive`
  (`|PlayMontage` (`self.m_skeletalMeshComponent`) "/Game/Blueprints/Animation/AI/Apostle_lvl1/Montages/Revive_Montage.Revive_Montage"))

(fn `GetPlayer`
  (bind _asro_dgame_mode (cast `/Game/Blueprints/RoDGameMode` (`GameplayStatics.GetGameMode`)))
  (bind _returnvalue (`RhythmOfTheDemonGameModeBase.GetPlayer` _asro_dgame_mode))
  (set `self.Player` _returnvalue))

(fn `PlayAnimationFromBrickType`
  (params (Brick :type "AbstractBrick Object Reference"))
  (bind _animationblueprint (`self.AnimationBlueprint`))
  (bind _animationblueprint_2 (`self.AnimationBlueprint`))
  (bind _asabstract_projectile (cast `AbstractProjectile` Brick)
    (:`then`
      (cast `/Game/Blueprints/Bricks/Projectile/ProjectileA` _asabstract_projectile
        (:`then`
          (`/Game/Blueprints/Animation/AI/Apostle_lvl1/AnimationBlueprint_apostle_lvl1.CastRightProj` _animationblueprint_2))
        (:`CastFailed`
          (cast `/Game/Blueprints/Bricks/Projectile/ProjectileB` _asabstract_projectile)
          (`/Game/Blueprints/Animation/AI/Apostle_lvl1/AnimationBlueprint_apostle_lvl1.CastLeftProj` _animationblueprint_2))))
    (:`CastFailed`
      (bind _asabstract_dodgeable_brick (cast `AbstractDodgeableBrick` Brick))
      (cast `/Game/Blueprints/Bricks/Dodgable/VerticalDodgeBrick` _asabstract_dodgeable_brick
        (:`then`
          (`/Game/Blueprints/Animation/AI/Apostle_lvl1/AnimationBlueprint_apostle_lvl1.CastHorizontalObstacle` _animationblueprint))
        (:`CastFailed`
          (cast `/Game/Blueprints/Bricks/Dodgable/HorizontalDodgeBrick` _asabstract_dodgeable_brick)
          (`/Game/Blueprints/Animation/AI/Apostle_lvl1/AnimationBlueprint_apostle_lvl1.CastVerticalObstacle` _animationblueprint))))))

(fn `UserConstructionScript`)